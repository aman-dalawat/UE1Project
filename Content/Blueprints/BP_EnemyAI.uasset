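; BP_EnemyAI is an enemy that chases the player and knocks characters back with a melee attack.
; Seeing a pawn through PawnSensing starts an AI move toward the player, and arrival plays an attack montage, gated by CanAttack until it completes or is interrupted.
; A forward sphere trace, run at montage start and on each notify begin, launches the hit character forward and upward without applying damage.
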(event OnSeePawn(PawnSensing)
  (params (Pawn :type Pawn%20Object%20Reference))
  (CallFunction|ChasePlayer))

(event Custom|Chase%20Player
  (bind _returnvalue (Transformation|GetActorLocation))
  (AI|AIMoveTo self "0, 0, 0" (Game|GetPlayerCharacter 0) 1.2e+02 false
    (:OnSuccess
      (if (Variables|Default|GetcanAttack?)
        (Animation|Montage|PlayMontage (Variables|Character|GetMesh) "/Game/Characters/Animations/Attack/A_Attack_Montage.A_Attack_Montage"
          (:then
            (Variables|Default|SetcanAttack? false)
            (bind (_outhit _returnvalue_2) (Collision|SphereTraceByChannel _returnvalue (+ _returnvalue (* (Math|Vector|GetForwardVector (Transformation|GetActorRotation)) 1.5e+02)) 25.0 "TraceTypeQuery3" false 0 "None" true "(R=1.000000,G=0.000000,B=0.000000,A=1.000000)" "(R=0.000000,G=1.000000,B=0.000000,A=1.000000)" 0.5 :!label _label))
            (if _returnvalue_2
              (bind _ascharacter (Utilities|Casting|CastToCharacter (.HitActor (Collision|BreakHitResult _outhit))))
              (Character|LaunchCharacter _ascharacter (+ (* (Math|Vector|GetForwardVector (Transformation|GetActorRotation)) (Variables|Default|GetfrontalKnockBack)) (Math|Vector|MakeVector 0.0 0.0 (Variables|Default|GetupwardKnockBack))) false false)))
          (:OnCompleted
            (Variables|Default|SetcanAttack? true :!label _label_2))
          (:OnInterrupted
            (goto _label_2))
          (:OnNotifyBegin
            (goto _label)))))))

(event EventBeginPlay)

(fn ConstructionScript)